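; BP_ItemSpawner is an actor that keeps one randomly chosen item spawned at its own location.
; BeginPlay and every Tick call AttemptToSpawn, which runs SpawnItem whenever CurrentItem is no longer valid, so replacement is immediate.
; SpawnItem picks a class from ItemsToSpawn, using the array length as the inclusive random maximum, so the index can fall out of range.
; An unconnected timer node leaves respawns without any delay.
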(event `self.ReceiveBeginPlay`
  (`self.AttemptToSpawn` :!label _label))

(event `self.ReceiveTick`
  (params (DeltaSeconds :type "Float (single-precision)"))
  (goto _label))

(fn `AttemptToSpawn`
  (`/Engine/EditorBlueprintResources/StandardMacros.IsValid` (`self.CurrentItem`)
    (:`Is Not Valid`
      (`self.SpawnItem`))))

(fn `SpawnItem`
  (bind _returnvalue (`|SpawnActorFromClass` (`|GetArrayItem` (`self.ItemsToSpawn`) (`KismetMathLibrary.RandomIntegerInRange` 0 (`KismetArrayLibrary.Array_Length` (`self.ItemsToSpawn`)))) (`KismetMathLibrary.MakeTransform` (`self.K2_GetActorLocation`) (`self.K2_GetActorRotation`)) "AdjustIfPossibleButAlwaysSpawn" "OverrideRootScale" null null))
  (set `self.CurrentItem` _returnvalue))

(fn `UserConstructionScript`)