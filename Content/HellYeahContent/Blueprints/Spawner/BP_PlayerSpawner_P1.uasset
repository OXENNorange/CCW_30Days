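; Spawner actor for player one that places a Player1 at its own location and rotation.
; AttemptToSpawn calls SpawnPlayer only when CurrentPlayer1 is invalid, and otherwise just prints a debug string.
; SpawnPlayer sets player character 0 as the new actor's owner and stores it in CurrentPlayer1.
; The event graph is empty, so nothing in this Blueprint triggers spawning by itself.
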(fn `AttemptToSpawn`
  (`/Engine/EditorBlueprintResources/StandardMacros.IsValid` (`self.CurrentPlayer1`)
    (:`Is Valid`
      (`KismetSystemLibrary.PrintString` "P1spawn"))
    (:`Is Not Valid`
      (`self.SpawnPlayer`))))

(fn `SpawnPlayer`
  (bind _returnvalue (`|SpawnActorFromClass` (`self.Player1`) (`KismetMathLibrary.MakeTransform` (`self.K2_GetActorLocation`) (`self.K2_GetActorRotation`)) "Undefined" "OverrideRootScale" (`GameplayStatics.GetPlayerCharacter` 0) null))
  (set `self.CurrentPlayer1` _returnvalue))

(fn `UserConstructionScript`)